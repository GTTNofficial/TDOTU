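; Base enemy with health and a simple player-follow behaviour, using a sprite and a health bar widget.
; While enabled and no player overlaps its Vicinity, Tick moves it toward the player along X via SetActorLocation, without sweep.
; Damage and healing functions update the EnemyHealth widget.
; Death stops following, spawns a coin one time in four and destroys the actor after a short delay; older movement and sprite-flip logic sits unused.
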(event EventTakeDamage
  (params (Damage :type Float%20%28single-precision%29) (DamageType :type DamageType%20Enum :default "NewEnumerator0") (HitInfo :type Hit%20Result%20Structure))
  (bind _dead_ (CallFunction|SubtractHealth Damage))
  (if _dead_
    (CallFunction|Die HitInfo)
    (Utilities|FlowControl|Delay 1.3)
    (Actor|DestroyActor)))

(event EventTick
  (params (DeltaSeconds :type Float%20%28single-precision%29))
  (bind _returnvalue (Transformation|GetActorLocation))
  (bind (_x _y _z) (Math|Vector|BreakVector _returnvalue))
  (if (and (== (Utilities|Array|Length (Collision|GetOverlappingActors (Variables|Default|GetVicinity) "/Game/Blueprint/Characters/Generic/BasePlayerCharacter.BasePlayerCharacter_C" :!class /Script/Engine.PrimitiveComponent)) 0) (Variables|Default|GetSimpleFollowPlayer?))
    (Transformation|SetActorLocation (Math|Vector|MakeVector (.X (Math|Vector|BreakVector (+ (* (* (Math|Vector|Normalize (- (Transformation|GetActorLocation (Game|GetPlayerCharacter 0)) _returnvalue)) DeltaSeconds) (Variables|Default|GetSpeed)) _returnvalue))) _y _z) false false)))

(fn ConstructionScript)

(fn SubtractHealth
  (params (Health :type Float%20%28single-precision%29))
  (bind _output_get (Variables|Default|SetHealth (- (Variables|Default|GetHealth) Health)))
  (CallFunction|UpdateHealthBar)
  (if (<= _output_get 0.0)
    (return true true)
    (else
      (return true false))))

(fn AddHealth
  (params (Health :type Float%20%28single-precision%29))
  (if (> (+ Health (Variables|Default|GetHealth)) (Variables|Default|GetMaxHealth))
    (Variables|Default|SetHealth (Variables|Default|GetMaxHealth))
    (else
      (Variables|Default|SetHealth (+ Health (Variables|Default|GetHealth)))))
  (CallFunction|UpdateHealthBar)
  (return true))

(fn Die
  (params (HitInfo :type Hit%20Result%20Structure))
  (Variables|Default|SetSimpleFollowPlayer? false)
  (if (and (Math|Random|RandomBool) (Math|Random|RandomBool))
    (Game|SpawnActorfromClass "/Game/Blueprint/Generic/Coins/B_Coin.B_Coin_C" (Math|Transform|MakeTransform (Transformation|GetWorldLocation (Variables|Default|GetSprite)) "0, 0, 0" "1,1,1") "Undefined" 0 0)
    (return true)))

(fn UpdateHealthBar
  (bind _asenemy_health (Utilities|Casting|CastToEnemyHealth (UserInterface|GetUserWidgetObject (Variables|Default|GetHealthBar))))
  (Default|UpdateHealthBar _asenemy_health (Variables|Default|GetHealth)))